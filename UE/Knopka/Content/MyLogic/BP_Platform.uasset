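; BP_Platform is a trigger platform that counts how many times the ThirdPersonCharacter steps onto it.
; Each overlap of its Box by that character increments StepCounter.
; It then looks up actors implementing BPI_PlatformTrigger and passes them the count through the PlatformIsTriggeredMessage interface call, avoiding references to specific receiver classes.
; Tick prints the running count on screen every frame as a Russian-language message.
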(event OnComponentBeginOverlap(Box)
  (params (OverlappedComponent :type Primitive%20Component%20Object%20Reference) (OtherActor :type Actor%20Object%20Reference) (OtherComp :type Primitive%20Component%20Object%20Reference) (OtherBodyIndex :type Integer) (bFromSweep :type Boolean) (SweepResult :type Hit%20Result%20Structure%20%28by%20ref%29))
  (Utilities|Casting|CastToThirdPersonCharacter OtherActor)
  (Variables|Default|SetStepCounter (+ (Variables|Default|GetStepCounter) 1))
  ;[1 1 1] Get a copy - удалить его и подключить напрямую
  (bind _outactors (Actor|GetAllActorswithInterface "/Game/MyLogic/BPI_PlatformTrigger.BPI_PlatformTrigger_C"))
  (Class|BPIPlatformTrigger|PlatformIsTriggered(Message) _outactors (Variables|Default|GetStepCounter)))

(event EventTick
  (params (DeltaSeconds :type Float%20%28single-precision%29))
  (Development|PrintString (Utilities|String|Append "Мы наступили на платформу " (Utilities|String|ToString(Integer) (Variables|Default|GetStepCounter)) " раз") true true "(R=0.000000,G=0.660000,B=1.000000,A=1.000000)" DeltaSeconds))

(fn ConstructionScript)