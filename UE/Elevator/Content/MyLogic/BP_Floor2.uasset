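; BP_Floor2 is an elevator actor that moves its Floor2 component vertically between three preset floor heights.
; When the player character overlaps its Box, it broadcasts ToFloorNumber2 to every actor implementing the BPI_Floor interface.
; The ElevatoronFloor event stores the previous height, starts a timeline and selects the target height from the floor number.
; Tick lerps between the two heights using the timeline alpha, keeping a hardcoded world X and Y.
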(event OnComponentBeginOverlap(Box)
  (params (OverlappedComponent :type Primitive%20Component%20Object%20Reference) (OtherActor :type Actor%20Object%20Reference) (OtherComp :type Primitive%20Component%20Object%20Reference) (OtherBodyIndex :type Integer) (bFromSweep :type Boolean) (SweepResult :type Hit%20Result%20Structure%20%28by%20ref%29))
  (Utilities|Casting|CastToThirdPersonCharacter OtherActor)
  (bind _outactors (Actor|GetAllActorswithInterface "/Game/MyLogic/BPI_Floor.BPI_Floor_C"))
  (Class|BPIFloor|ElevatoronFloor(Message) _outactors (Variables|Default|GetToFloorNumber2)))

(event EventElevatoronFloor
  (params (FloorNumber :type Integer))
  (Variables|Default|SetPreHight2 (Variables|Default|GetHight2))
  (bind _alpha (Timeline|Timeline_0 PlayFromStart)
    (:Update
      (if (== FloorNumber 1)
        (Variables|Default|SetHight2 330)
        (elif (== FloorNumber 2)
          (Variables|Default|SetHight2 1070)
          (elif (== FloorNumber 3)
            (Variables|Default|SetHight2 1860)))))))

(event EventTick
  (params (DeltaSeconds :type Float%20%28single-precision%29))
  (Transformation|SetWorldLocation (Variables|Default|GetFloor2) (Math|Vector|MakeVector 4.2e+02 1.02e+03 (Math|Float|Lerp (Math|Conversions|ToFloat(Integer) (Variables|Default|GetPreHight2)) (Math|Conversions|ToFloat(Integer) (Variables|Default|GetHight2)) (stale EventElevatoronFloor _alpha))) false false))

(fn ConstructionScript)