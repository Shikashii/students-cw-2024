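; Elevator call button that reports a floor number through the BPI_Floor interface.
; At BeginPlay and whenever a ThirdPersonCharacter overlaps its Box, it sends FloorNumber1 via ElevatorOnFloorMessage to actors implementing that interface.
; Every Tick it prints a Russian on-screen message giving the elevator's current floor from FloorNumber.
; Its own ElevatoronFloor event has no logic attached.
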(event OnComponentBeginOverlap(Box)
  (params (OverlappedComponent :type Primitive%20Component%20Object%20Reference) (OtherActor :type Actor%20Object%20Reference) (OtherComp :type Primitive%20Component%20Object%20Reference) (OtherBodyIndex :type Integer) (bFromSweep :type Boolean) (SweepResult :type Hit%20Result%20Structure%20%28by%20ref%29))
  (Utilities|Casting|CastToThirdPersonCharacter OtherActor)
  (bind _outactors (Actor|GetAllActorswithInterface "/Game/MyLogic/BPI_Floor.BPI_Floor_C"))
  (Class|BPIFloor|ElevatoronFloor(Message) _outactors (Variables|Default|GetFloorNumber1)))

(event EventElevatoronFloor
  (params (FloorNumber :type Integer)))

(event EventBeginPlay
  (bind _outactors (Actor|GetAllActorswithInterface "/Game/MyLogic/BPI_Floor.BPI_Floor_C"))
  (Class|BPIFloor|ElevatoronFloor(Message) _outactors (Variables|Default|GetFloorNumber1)))

(event EventTick
  (params (DeltaSeconds :type Float%20%28single-precision%29))
  (Development|PrintString (Utilities|String|Append "Сейчас лифт находится на этаже номер " (Utilities|String|ToString(Integer) (stale EventElevatoronFloor FloorNumber))) true true "(R=0.000000,G=0.660000,B=1.000000,A=1.000000)" DeltaSeconds))

(fn ConstructionScript)