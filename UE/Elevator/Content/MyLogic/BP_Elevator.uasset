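; BP_Elevator is an elevator Blueprint that moves its Elevator component between three floors, each with a hard-coded height.
; The ElevatoronFloor event stores the current target height as the previous one, plays a timeline from the start and sets the new height from the floor number during timeline updates.
; Tick lerps between the two heights by the timeline alpha and sets the world location at fixed X and Y coordinates.
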(event EventElevatoronFloor
  (params (FloorNumber :type Integer))
  (Variables|Default|SetPreHight (Variables|Default|GetHight))
  (bind _alpha (Timeline|Timeline_0 PlayFromStart)
    (:Update
      (if (== FloorNumber 1)
        (Variables|Default|SetHight 230)
        (elif (== FloorNumber 2)
          (Variables|Default|SetHight 970)
          (elif (== FloorNumber 3)
            (Variables|Default|SetHight 1760)))))))

(event EventTick
  (params (DeltaSeconds :type Float%20%28single-precision%29))
  (Transformation|SetWorldLocation (Variables|Default|GetElevator) (Math|Vector|MakeVector 4.2e+02 7.8e+02 (Math|Float|Lerp (Math|Conversions|ToFloat(Integer) (Variables|Default|GetPreHight)) (Math|Conversions|ToFloat(Integer) (Variables|Default|GetHight)) (stale EventElevatoronFloor _alpha))) false false))

(fn ConstructionScript)